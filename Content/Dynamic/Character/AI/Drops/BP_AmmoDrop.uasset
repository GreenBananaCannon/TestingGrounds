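; BP_AmmoDrop is an ammo pickup that refills the player's gun on touch.
; An overlap on its ItemCollider passes through an IsPlayer check, which compares the overlapping actor to player character 0.
; On a match it casts player pawn 0 to Mannequin, adds AmmoContained to that pawn's Gun through IncreaseAmmo, then destroys itself.
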(event OnComponentBeginOverlap(ItemCollider)
  (params (OverlappedComponent :type Primitive%20Component%20Object%20Reference) (OtherActor :type Actor%20Object%20Reference) (OtherComp :type Primitive%20Component%20Object%20Reference) (OtherBodyIndex :type Integer) (bFromSweep :type Boolean) (SweepResult :type Hit%20Result%20Structure%20%28by%20ref%29))
  (Utilities|IsPlayer OtherActor
    (:true
      (bind _asmannequin (Utilities|Casting|CastToMannequin (Game|Player|GetPlayerPawn 0)))
      (Class|Gun|IncreaseAmmo (Variables|/Script/TestingGrounds.Mannequin|GetGun _asmannequin) (Variables|Default|GetAmmoContained))
      (Actor|DestroyActor))))

(fn ConstructionScript)