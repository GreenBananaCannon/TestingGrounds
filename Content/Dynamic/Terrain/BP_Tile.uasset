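; Terrain tile for an infinite-terrain game mode that scatters rocks, boxes, containers and canisters via PlaceActors on BeginPlay.
; Its gate starts locked and red, turning passable and green while the player overlaps LockingVolume.
; Leaving that volume relocks the gate and asks InfiniteTerrainGameMode to spawn another tile, with GetAttachLocation exposing the AttachPoint transform.
; The player entering GarbageCollectorVolume destroys the tile.
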(event OnComponentBeginOverlap(LockingVolume)
  (params (OverlappedComponent :type Primitive%20Component%20Object%20Reference) (OtherActor :type Actor%20Object%20Reference) (OtherComp :type Primitive%20Component%20Object%20Reference) (OtherBodyIndex :type Integer) (bFromSweep :type Boolean) (SweepResult :type Hit%20Result%20Structure%20%28by%20ref%29))
  (Utilities|IsPlayer OtherActor)
  (CallFunction|Unlock))

(event OnComponentEndOverlap(LockingVolume)
  (params (OverlappedComponent :type Primitive%20Component%20Object%20Reference) (OtherActor :type Actor%20Object%20Reference) (OtherComp :type Primitive%20Component%20Object%20Reference) (OtherBodyIndex :type Integer))
  (Utilities|IsPlayer OtherActor)
  (CallFunction|Lock)
  (bind _asinfinite_terrain_game_mode (Utilities|Casting|CastToInfiniteTerrainGameMode (Game|GetGameMode)))
  (Default|SpawnTile _asinfinite_terrain_game_mode))

(event OnComponentBeginOverlap(GarbageCollectorVolume)
  (params (OverlappedComponent :type Primitive%20Component%20Object%20Reference) (OtherActor :type Actor%20Object%20Reference) (OtherComp :type Primitive%20Component%20Object%20Reference) (OtherBodyIndex :type Integer) (bFromSweep :type Boolean) (SweepResult :type Hit%20Result%20Structure%20%28by%20ref%29))
  (Utilities|IsPlayer OtherActor)
  (Actor|DestroyActor))

(event EventBeginPlay
  ;[1 1 1] Begin play happening after Locking volume overlap!
  (CallFunction|Lock)
  (Class|Tile|PlaceActors "/Game/Dynamic/Terrain/Props/BP_Rock03.BP_Rock03_C" 1 5 2.5e+02 1.0 3.0)
  (Class|Tile|PlaceActors "/Game/Dynamic/Terrain/Props/BP_BoxStack.BP_BoxStack_C" 3 5 175.0 1.0 1.0)
  (Class|Tile|PlaceActors "/Game/Dynamic/Terrain/Props/BP_Container.BP_Container_C" 3 3 4e+02 1.0 1.0)
  (Class|Tile|PlaceActors "/Game/Dynamic/Terrain/Props/BP_Canister.BP_Canister_C" 3 7 5e+01 1.0 1.0)
  (Class|Tile|PlaceActors "/Game/Dynamic/Terrain/Props/BP_Rock02.BP_Rock02_C" 1 5 2e+02 1.0 2.0)
  (Class|Tile|PlaceActors "/Game/Dynamic/Terrain/Props/BP_Box.BP_Box_C" 1 5 1e+02 1.0 1.0))

(fn ConstructionScript)

(fn GetAttachLocation
  (return (Transformation|GetWorldTransform (Variables|Default|GetAttachPoint))))

(fn Unlock
  (Collision|SetCollisionEnabled (Variables|Default|GetGate) "NoCollision")
  (Rendering|Material|SetMaterial (Variables|Default|GetGate) 0 "/Game/Dynamic/Terrain/MI_Barrier_Green.MI_Barrier_Green")
  (Development|PrintString "Gate Set to Green"))

(fn Lock
  (Collision|SetCollisionEnabled (Variables|Default|GetGate) "QueryAndPhysics")
  (Rendering|Material|SetMaterial (Variables|Default|GetGate) 0 "/Game/Dynamic/Terrain/MI_Barrier_Red.MI_Barrier_Red"))